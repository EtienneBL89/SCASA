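; BP_ZipLine is a spline-based zipline actor that the first-person character can use.
; The construction script places Start and End at the spline's ends through a capsule half-height offset helper, builds spline mesh segments along it and assigns the endpoint meshes.
; Overlapping Start passes the spline and play rate to FirstPersonCharacter, and leaving notifies it that the zipline is out of range.
; The actor itself contains no ride movement logic.
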(event `self.ReceiveBeginPlay`)

(event `self.Start.OnComponentBeginOverlap`
  (params (OverlappedComponent :type "PrimitiveComponent Object Reference") (OtherActor :type "Actor Object Reference") (OtherComp :type "PrimitiveComponent Object Reference") (OtherBodyIndex :type Integer) (bFromSweep :type Boolean) (SweepResult :type "HitResult Structure (by ref)"))
  (bind _asfirst_person_character (cast `/Game/Blueprints/FirstPersonCharacter` OtherActor))
  (`/Game/Blueprints/FirstPersonCharacter.ZiplineInRange` _asfirst_person_character (`self.Zipline`) (`self.PlayRate`)))

(event `self.Start.OnComponentEndOverlap`
  (params (OverlappedComponent :type "PrimitiveComponent Object Reference") (OtherActor :type "Actor Object Reference") (OtherComp :type "PrimitiveComponent Object Reference") (OtherBodyIndex :type Integer))
  (bind _asfirst_person_character (cast `/Game/Blueprints/FirstPersonCharacter` OtherActor))
  (`/Game/Blueprints/FirstPersonCharacter.ZiplineOutOfRange` _asfirst_person_character))

(fn `UserConstructionScript`
  (bind _zipline (`self.Zipline`))
  (bind _zipline_2 (`self.Zipline`))
  (bind _returnvalue (`SplineComponent.GetNumberOfSplinePoints` _zipline))
  (`|ExecutionSequence`
    (:`then_0`
      ;[1 1 1] Set start and end location
      (`SceneComponent.K2_SetRelativeLocation` (`self.End`) (`self.OffsetByCapsuleHalfHeight` (`SplineComponent.GetLocationAtSplinePoint` _zipline _returnvalue "Local")) false false)
      (`SceneComponent.K2_SetRelativeLocation` (`self.Start`) (`self.OffsetByCapsuleHalfHeight` (`SplineComponent.GetLocationAtSplinePoint` _zipline 0 "Local")) false false))
    (:`then_1`
      ;[1 1 1] Add spline meshes
      (for _index (range (+ _returnvalue 1))
        (bind _returnvalue_2 (`AddComponent|NODE_AddSplineMeshComponent-0`))
        (`SceneComponent.K2_AttachToComponent` (`self.DefaultSceneRoot`) _returnvalue_2 "None" "KeepRelative" "KeepRelative" "KeepRelative" true)
        (bind (_location _tangent) (`SplineComponent.GetLocationAndTangentAtSplinePoint` _zipline_2 _index "Local"))
        (bind (_location_2 _tangent_2) (`SplineComponent.GetLocationAndTangentAtSplinePoint` _zipline_2 (+ _index 1) "Local"))
        (`SplineMeshComponent.SetStartAndEnd` _returnvalue_2 _location _tangent _location_2 _tangent_2 true)))
    (:`then_2`
      ;[1 1 1] Set meshes for start and end
      (`StaticMeshComponent.SetStaticMesh` (`self.Mesh 1`) (`self.Mesh`))
      (`StaticMeshComponent.SetStaticMesh` (`self.Mesh 2`) (`self.Mesh`)))))