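; Climbable ladder actor that notifies FirstPersonCharacter when it enters or leaves the ladder's detection box.
; The construction script stacks LadderHeight instances of BaseMesh vertically in world space with zero rotation, spacing them by mesh height.
; It then sizes and centers PlayerDetector over the stack and stores TopLocation and BoxLocation for the character.
; Overlap events pass the ladder to LadderInRange and call LadderOutOfRange on exit.
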(event `self.PlayerDetector.OnComponentBeginOverlap`
  (params (OverlappedComponent :type "PrimitiveComponent Object Reference") (OtherActor :type "Actor Object Reference") (OtherComp :type "PrimitiveComponent Object Reference") (OtherBodyIndex :type Integer) (bFromSweep :type Boolean) (SweepResult :type "HitResult Structure (by ref)"))
  (bind _asfirst_person_character (cast `/Game/Blueprints/Player/FirstPersonCharacter` OtherActor))
  (`/Game/Blueprints/Player/FirstPersonCharacter.LadderInRange` _asfirst_person_character self))

(event `self.PlayerDetector.OnComponentEndOverlap`
  (params (OverlappedComponent :type "PrimitiveComponent Object Reference") (OtherActor :type "Actor Object Reference") (OtherComp :type "PrimitiveComponent Object Reference") (OtherBodyIndex :type Integer))
  (bind _asfirst_person_character (cast `/Game/Blueprints/Player/FirstPersonCharacter` OtherActor))
  (`/Game/Blueprints/Player/FirstPersonCharacter.LadderOutOfRange` _asfirst_person_character))

(fn `UserConstructionScript`
  (bind (_returnvalue_x _returnvalue_y) (`KismetMathLibrary.BreakVector` (`self.K2_GetActorLocation`)))
  (bind _playerdetector (`self.PlayerDetector`))
  (bind (_min _max) (`StaticMeshComponent.GetLocalBounds` (`self.BaseMesh`)))
  (bind _returnvalue (- (`self.NewInstanceZOffset`) (/ (`self.GetMeshHeight`) 2.0)))
  (bind _returnvalue_2 (/ _returnvalue 2.0))
  (`|ExecutionSequence`
    (:`then_0`
      ;[1 1 1] Initialize NewInstanceZOffset
      (set `self.NewInstanceZOffset` (/ (`self.GetMeshHeight`) 2.0)))
    (:`then_1`
      ;[1 1 1] Create meshes according to LadderHeight
      (for _ (range 1 (+ (`self.LadderHeight`) 1))
        (`InstancedStaticMeshComponent.AddInstanceWorldSpace` (`self.BaseMesh`) (`KismetMathLibrary.MakeTransform` (`KismetMathLibrary.MakeVector` (.x (`self.K2_GetActorLocation`)) (.y (`self.K2_GetActorLocation`)) (+ (.z (`self.K2_GetActorLocation`)) (`self.NewInstanceZOffset`)))))
        (set `self.NewInstanceZOffset` (+ (`self.NewInstanceZOffset`) (`self.GetMeshHeight`))))
      ;[1 1 1] Set PlayerDetector extent and relative transform
      (`BoxComponent.SetBoxExtent` _playerdetector (`KismetMathLibrary.MakeVector` (/ (- (.x _max) (.x _min)) 2.0) (/ (- (.y _max) (.y _min)) 2.0) _returnvalue_2) true)
      (`SceneComponent.K2_SetRelativeTransform` _playerdetector (`KismetMathLibrary.MakeTransform` (`KismetMathLibrary.MakeVector` 0.0 0.0 _returnvalue_2)) false false)
      ;[1 1 1] Set variables for PlayerCharacter
      (set `self.TopLocation` (`KismetMathLibrary.MakeVector` _returnvalue_x _returnvalue_y _returnvalue))
      (set `self.BoxLocation` (`SceneComponent.K2_GetComponentLocation` (`self.PlayerDetector`))))))