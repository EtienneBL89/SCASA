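; BP_Ladder is a climbable ladder actor that tells the first-person character when it is within reach.
; The construction script stacks vertical BaseMesh instances according to LadderHeight, then sizes and centers the PlayerDetector box along the stack.
; It also stores TopLocation and BoxLocation.
; Overlapping the box passes the ladder to FirstPersonCharacter through LadderInRange, and leaving calls LadderOutOfRange.
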(event `self.PlayerDetector.OnComponentBeginOverlap`
  (params (OverlappedComponent :type "PrimitiveComponent Object Reference") (OtherActor :type "Actor Object Reference") (OtherComp :type "PrimitiveComponent Object Reference") (OtherBodyIndex :type Integer) (bFromSweep :type Boolean) (SweepResult :type "HitResult Structure (by ref)"))
  (bind _asfirst_person_character (cast `/Game/Blueprints/FirstPersonCharacter` OtherActor))
  (`/Game/Blueprints/FirstPersonCharacter.LadderInRange` _asfirst_person_character self))

(event `self.PlayerDetector.OnComponentEndOverlap`
  (params (OverlappedComponent :type "PrimitiveComponent Object Reference") (OtherActor :type "Actor Object Reference") (OtherComp :type "PrimitiveComponent Object Reference") (OtherBodyIndex :type Integer))
  (bind _asfirst_person_character (cast `/Game/Blueprints/FirstPersonCharacter` OtherActor))
  (`/Game/Blueprints/FirstPersonCharacter.LadderOutOfRange` _asfirst_person_character))

(fn `UserConstructionScript`
  (bind (_returnvalue_x _returnvalue_y) (`KismetMathLibrary.BreakVector` (`self.K2_GetActorLocation`)))
  (bind _playerdetector (`self.PlayerDetector`))
  (bind _returnvalue (- (`self.NewInstanceZOffset`) 50.0))
  (bind _returnvalue_2 (/ _returnvalue 2.0))
  ;[1 0 0] TODO: Make more procedural later
  (for _ (range 1 (+ (`self.LadderHeight`) 1))
    (`InstancedStaticMeshComponent.AddInstanceWorldSpace` (`self.BaseMesh`) (`KismetMathLibrary.MakeTransform` (`KismetMathLibrary.MakeVector` (.x (`self.K2_GetActorLocation`)) (.y (`self.K2_GetActorLocation`)) (+ (.z (`self.K2_GetActorLocation`)) (`self.NewInstanceZOffset`)))))
    (set `self.NewInstanceZOffset` (+ (`self.NewInstanceZOffset`) 100.0)))
  (`BoxComponent.SetBoxExtent` _playerdetector (`KismetMathLibrary.MakeVector` 50.0 50.0 _returnvalue_2) true)
  (`SceneComponent.K2_SetRelativeTransform` _playerdetector (`KismetMathLibrary.MakeTransform` (`KismetMathLibrary.MakeVector` 0.0 0.0 _returnvalue_2) (struct) (1.0 1.0 1.0)) false false)
  (set `self.TopLocation` (`KismetMathLibrary.MakeVector` _returnvalue_x _returnvalue_y _returnvalue))
  (set `self.BoxLocation` (`SceneComponent.K2_GetComponentLocation` (`self.PlayerDetector`))))