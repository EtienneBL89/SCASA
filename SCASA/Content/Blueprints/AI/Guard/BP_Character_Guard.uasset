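; Enemy guard character that aims at, shoots and reloads against the player, and ragdolls when damaged.
; Tick reads blackboard range and sight flags to interpolate aim pitch and yaw for the animation blueprint, and eases walk speed through a gate.
; FireRifle checks line of sight from the muzzle, then spawns a projectile toward the player after a delay.
; Damage runs once, unpossessing the guard and dropping the gun; game over stops shooting.
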(event `self.ReceiveBeginPlay`
  (set `self.CurrentAmmo` (`self.MaxAmmo`))
  (add `/Game/Blueprints/Player/FirstPersonGameMode.GameOver` (cast `/Game/Blueprints/Player/FirstPersonGameMode` (`GameplayStatics.GetGameMode`) :!pure true) (delegate `StopShooting`)))

(event `StopShooting`
  ;[1 0 0] TODO: Improve on this
  (set `self.IsPlayerAlive` false))

(event `self.ReceiveTick`
  (params (DeltaSeconds :type "Float (single-precision)"))
  (bind _returnvalue (`AIBlueprintHelperLibrary.GetBlackboard` null))
  (bind _charactermovement (`self.CharacterMovement`))
  (bind _maxwalkspeed (`CharacterMovementComponent.MaxWalkSpeed` _charactermovement))
  (if (`|EnumInequality` (`self.Status`) "NewEnumerator5")
    (`|ExecutionSequence`
      (:`then_0`
        ;[1 1 1] Get the pitch and yaw values for the animation blueprint
        (if (and (`BlackboardComponent.GetValueAsBool` _returnvalue "IsPlayerInRange") (`BlackboardComponent.GetValueAsBool` _returnvalue "CanSeePlayer"))
          (`|ExecutionSequence`
            (:`then_0`
              (bind (_pitch _yaw) (`self.CalculateAimPitchAndAimYaw` (`self.K2_GetActorLocation` (`GameplayStatics.GetPlayerCharacter` 0)) DeltaSeconds 30.0))
              (set `self.AimPitch` _pitch)
              (set `self.AimYaw` _yaw)))
          (elif (not (`KismetMathLibrary.NearlyEqual_FloatFloat` (+ (`self.AimYaw`) (`self.AimPitch`)) 0.0 1.0))
            (`self.ResetAimPitchAndYaw` DeltaSeconds 4.0))))
      (:`then_1`
        ;[1 1 1] Change the guard's walking speed
        (`/Engine/EditorBlueprintResources/StandardMacros.Gate` true :!label _label
          (:`Exit`
            (set `CharacterMovementComponent.MaxWalkSpeed` (`KismetMathLibrary.Lerp` _maxwalkspeed (stale `UpdateSpeed` NewSpeed) (* DeltaSeconds 8.0)) _charactermovement)
            (if (`KismetMathLibrary.NearlyEqual_FloatFloat` _maxwalkspeed (stale `UpdateSpeed` NewSpeed) 1.0)
              (`self.SpeedUpdated`))))))))

(event `UpdateSpeed`
  (params (NewSpeed :type "Float (double-precision)"))
  ;[1 1 1] Change the guard's walking speed
  (goto _label :!via `Open`))

(event `SpeedUpdated`
  ;[1 1 1] Change the guard's walking speed
  (goto _label :!via `Close`))

(event `/Game/Blueprints/Interfaces/ICombat.FireRifle`
  (bind _returnvalue (`SkeletalMeshComponent.GetAnimInstance` (`self.Mesh`)))
  (bind _location (.location (`SceneComponent.GetSocketTransform` (`self.Gun`) "Muzzle" "RTS_World")))
  ;[1 1 1] Combat events
  (if (`self.IsPlayerAlive`)
    (if (`Controller.LineOfSightTo` (`self.GetController`) (`GameplayStatics.GetPlayerCharacter` 0) (`SceneComponent.GetSocketLocation` (`self.Gun`) "Muzzle") false)
      (`KismetSystemLibrary.Delay` 0.5) ; Do not fire until aiming offset has been applied.
      (`/Engine/EditorBlueprintResources/StandardMacros.DecrementInt` (`self.CurrentAmmo`)
        (:`  `
          ;;[1 1 1] Play animations
          (if (not (`AnimInstance.Montage_IsPlaying` _returnvalue "/Game/Blueprints/AI/Guard/Animations/Fire_Rifle_Montage.Fire_Rifle_Montage"))
            (`AnimInstance.Montage_Play` _returnvalue "/Game/Blueprints/AI/Guard/Animations/Fire_Rifle_Montage.Fire_Rifle_Montage" 0.4 "MontageLength" 0.0 true) ; Play firing animation
            ;;[1 1 1] Play sounds
            (`GameplayStatics.PlaySoundAtLocation` "/Game/FirstPerson/Audio/FirstPersonTemplateWeaponFire02.FirstPersonTemplateWeaponFire02" (`self.K2_GetActorLocation`) (struct) 1.0 1.0 0.0 null null null) ; Play firing sound
            (`|SpawnActorFromClass` "/Game/Blueprints/Player/FirstPersonProjectile.FirstPersonProjectile_C" (`KismetMathLibrary.MakeTransform` (+ (* (`KismetMathLibrary.GetForwardVector` (`self.K2_GetActorRotation`)) 100.0) _location) (`KismetMathLibrary.FindLookAtRotation` _location (`self.K2_GetActorLocation` (`GameplayStatics.GetPlayerCharacter` 0))) (1.0 1.0 1.0)) "AlwaysSpawn" "OverrideRootScale" null self) ; Spawn projectile
          ))))))

(event `/Game/Blueprints/Interfaces/ICombat.Reload Rifle`
  (bind _returnvalue (`SkeletalMeshComponent.GetAnimInstance` (`self.Mesh`)))
  ;[1 1 1] Combat events
  (set `self.CurrentAmmo` (`self.MaxAmmo`))
  ;;[1 1 1] Play animations
  (if (not (`AnimInstance.Montage_IsPlaying` _returnvalue "/Game/Blueprints/AI/Guard/Animations/Reload_Rifle_Montage.Reload_Rifle_Montage"))
    (`AnimInstance.Montage_Play` _returnvalue "/Game/Blueprints/AI/Guard/Animations/Reload_Rifle_Montage.Reload_Rifle_Montage" 1.0 "MontageLength" 0.0 true) ; Play reloading animation
    ;;[1 1 1] Play sounds
    (`GameplayStatics.PlaySoundAtLocation` "/Game/Audio/S_ReloadRifle.S_ReloadRifle" (`self.K2_GetActorLocation`) (struct) 1.0 1.0 0.0 null null null) ; Play reloading sound
  ))

(event `/Game/Blueprints/Interfaces/ICombat.ReceiveDamage`
  (bind _gun (`self.Gun`))
  (bind _mesh (`self.Mesh`))
  ;[1 1 1] Combat events
  (`/Engine/EditorBlueprintResources/StandardMacros.DoOnce` false
    (:`Completed`
      (`Controller.UnPossess` (`self.GetController`))
      (`CharacterMovementComponent.DisableMovement` (`self.CharacterMovement`))
      (`|ExecutionSequence`
        (:`then_0`
          (`SceneComponent.K2_DetachFromComponent` _gun "KeepRelative" "KeepRelative" "KeepRelative" true)
          (`PrimitiveComponent.SetCollisionEnabled` _gun "QueryAndPhysics")
          (`PrimitiveComponent.SetSimulatePhysics` _gun true))
        (:`then_1`
          (`PrimitiveComponent.SetCollisionEnabled` _mesh "QueryAndPhysics")
          (`SkeletalMeshComponent.SetAllBodiesSimulatePhysics` _mesh true)
          (set `self.Status` "NewEnumerator5"))))))

(fn `CalculateAimPitchAndAimYaw`
  (params (Target :type "Vector Structure (by ref)") (DeltaTime :type "Float (double-precision)") (InterpSpeed :type "Float (double-precision)"))
  (returns (Pitch :type "Float (double-precision)") (Yaw :type "Float (double-precision)"))
  (return (`KismetMathLibrary.ClampAngle` (.pitch (`KismetMathLibrary.RInterpTo` (`KismetMathLibrary.MakeRotator` 0.0 (`self.AimPitch`) (`self.AimYaw`)) (`KismetMathLibrary.NormalizedDeltaRotator` (`KismetMathLibrary.FindLookAtRotation` (`self.K2_GetActorLocation`) Target) (`self.K2_GetActorRotation`)) DeltaTime InterpSpeed)) -90.0 90.0) (`KismetMathLibrary.ClampAngle` (.yaw (`KismetMathLibrary.RInterpTo` (`KismetMathLibrary.MakeRotator` 0.0 (`self.AimPitch`) (`self.AimYaw`)) (`KismetMathLibrary.NormalizedDeltaRotator` (`KismetMathLibrary.FindLookAtRotation` (`self.K2_GetActorLocation`) Target) (`self.K2_GetActorRotation`)) DeltaTime InterpSpeed)) -90.0 90.0)))

(fn `GetCurrentAmmo`
  (returns (CurrentAmmo :type Integer))
  (return (`self.CurrentAmmo`)))

(fn `ResetAimPitchAndYaw`
  (params (DeltaTime :type "Float (double-precision)") (InterpSpeed :type "Float (double-precision)"))
  (bind _returnvalue (* DeltaTime InterpSpeed))
  (set `self.AimPitch` (`KismetMathLibrary.Lerp` (`self.AimPitch`) 0.0 _returnvalue))
  (set `self.AimYaw` (`KismetMathLibrary.Lerp` (`self.AimYaw`) 0.0 _returnvalue)))

(fn `UserConstructionScript`)