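; AI controller for guard characters that sets up patrolling and player detection.
; On BeginPlay it runs BT_Guard and seeds the Blackboard with whether a patrol path exists and, if so, its default direction.
; PathIsLooping is always written as false for valid paths, leaving the path's own IsLooping unused.
; AI Perception updates set CanSeePlayer from whether the first-person player character was successfully sensed.
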(event `self.ReceiveBeginPlay`
  (bind _returnvalue (`AIBlueprintHelperLibrary.GetBlackboard` null))
  (bind _asbp_character_guard (cast `/Game/Blueprints/AI/Guard/BP_Character_Guard` (`self.K2_GetPawn`)))
  (bind _output_get (set `self.ControlledPawn` _asbp_character_guard))
  (`self.RunBehaviorTree` "/Game/Blueprints/AI/Guard/BT_Guard.BT_Guard")
  (bind _patrolpath (`/Game/Blueprints/AI/Guard/BP_Character_Guard.PatrolPath` _output_get)
    (:`then`
      (`BlackboardComponent.SetValueAsBool` _returnvalue "HasPath" true)
      (`BlackboardComponent.SetValueAsBool` _returnvalue "PathIsLooping" false)
      (`BlackboardComponent.SetValueAsEnum` _returnvalue "PathDirection" (`/Game/Blueprints/AI/Guard/Patrol/BP_PatrolPath.DefaultDirection` _patrolpath)))
    (:`else`
      (`BlackboardComponent.SetValueAsBool` _returnvalue "HasPath" false))))

(event `self.AIPerception.OnTargetPerceptionUpdated`
  (params (Actor :type "Actor Object Reference") (Stimulus :type "AIStimulus Structure"))
  (cast `/Game/Blueprints/Player/FirstPersonCharacter` Actor)
  (`BlackboardComponent.SetValueAsBool` (`AIBlueprintHelperLibrary.GetBlackboard` null) "CanSeePlayer" (`.bSuccessfullySensed` (break `AIStimulus` Stimulus))))

(fn `UserConstructionScript`)