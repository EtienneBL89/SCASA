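; BP_Distraction is a projectile that makes noise on impact to serve as a distraction.
; Each hit plays a thud and reports an AI noise event at the hit location, throttled by a DoOnce that resets after a short delay.
; Thud volume calls CalculateVolumeModifier, whose clamped vertical-speed calculation is left unused.
; When the projectile stops, it spawns a BP_DistractionPickUp in its place and destroys itself.
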(event `self.ReceiveTick`
  (params (DeltaSeconds :type "Float (single-precision)")))

(event `self.ReceiveHit`
  (params (MyComp :type "PrimitiveComponent Object Reference") (Other :type "Actor Object Reference") (OtherComp :type "PrimitiveComponent Object Reference") (bSelfMoved :type Boolean) (HitLocation :type "Vector Structure") (HitNormal :type "Vector Structure") (NormalImpulse :type "Vector Structure") (Hit :type "HitResult Structure (by ref)"))
  (`/Engine/EditorBlueprintResources/StandardMacros.DoOnce` false :!label _label
    (:`Completed`
      (`GameplayStatics.PlaySoundAtLocation` "/Game/Audio/S_Thud.S_Thud" HitLocation (struct) (`self.CalculateVolumeModifier`) 1.0 0.0 null null null)
      (`AISense_Hearing.ReportNoiseEvent` HitLocation 1.0 self 0.0 "Noise")
      (`KismetSystemLibrary.Delay` 0.2)
      (goto _label :!via `Reset`))))

(event `self.ProjectileMovement.OnProjectileStop`
  (params (ImpactResult :type "HitResult Structure (by ref)"))
  (`|SpawnActorFromClass` "/Game/Blueprints/PickUps/BP_DistractionPickUp.BP_DistractionPickUp_C" (`self.GetTransform`) "Undefined" "OverrideRootScale" null null)
  (`self.K2_DestroyActor`))

(fn `UserConstructionScript`)