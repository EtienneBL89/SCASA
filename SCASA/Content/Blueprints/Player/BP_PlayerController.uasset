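; Player controller Blueprint that handles level retry through the Retry input action.
; On BeginPlay it binds to the FirstPersonGameMode game-over event and caches the current level's name.
; A DoOnce node gates retry: game over resets it, and a Retry press that passes through it reopens the cached level.
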(event `self.ReceiveBeginPlay`
  (bind _asfirst_person_game_mode (cast `/Game/Blueprints/Player/FirstPersonGameMode` (`GameplayStatics.GetGameMode`)))
  (add `/Game/Blueprints/Player/FirstPersonGameMode.GameOver` _asfirst_person_game_mode (delegate `EnableRetryInput`))
  (bind _returnvalue (`GameplayStatics.GetCurrentLevelName` true))
  (set `self.LevelName` (`KismetStringLibrary.Conv_StringToName` _returnvalue)))

(event `EnableRetryInput`
  (goto _label :!via `Reset`))

(event `InputAction|Retry`
  (params (Key :type "Key Structure"))
  (:`Pressed`
    (`/Engine/EditorBlueprintResources/StandardMacros.DoOnce` false :!label _label
      (:`Completed`
        (`GameplayStatics.OpenLevel` (`self.LevelName`))))))

(fn `UserConstructionScript`)